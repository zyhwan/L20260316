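; BP_Balloon is a balloon actor that rises each Tick and recycles itself on passing a height limit.
; Movement adds Speed scaled by delta time to the up vector, rather than multiplying them, and offsets the location without sweep.
; Above MaxHigh, it spawns a replacement at a random low position with random Speed, then destroys itself.
; A mesh hit only prints a debug string.
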(event `self.ReceiveTick`
  (params (DeltaSeconds :type "Float (single-precision)"))
  (bind (_returnvalue_x _returnvalue_y _returnvalue_z) (`KismetMathLibrary.BreakVector` (`self.K2_GetActorLocation`)))
  (`self.K2_SetActorLocation` (+ (+ (* DeltaSeconds (`self.Speed`)) (`self.GetActorUpVector`)) (`self.K2_GetActorLocation`)))
  (if (> _returnvalue_z (`self.MaxHigh`))
    (bind _returnvalue (`|SpawnActorFromClass` "BP_Balloon_C" (`KismetMathLibrary.MakeTransform` (`KismetMathLibrary.MakeVector` (`KismetMathLibrary.RandomFloatInRange` -3800.0 3800.0) (`KismetMathLibrary.RandomFloatInRange` -3800.0 3800.0) (`KismetMathLibrary.RandomFloatInRange` 50.0 150.0))) "Undefined" "MultiplyWithRoot" null null))
    (set `/Game/Blueprints/Actor/BP_Balloon.Speed` (`KismetMathLibrary.RandomFloatInRange` 1.0 200.0) _returnvalue)
    (`self.K2_DestroyActor`)))

(event `self.StaticMesh.OnComponentHit`
  (params (HitComponent :type "PrimitiveComponent Object Reference") (OtherActor :type "Actor Object Reference") (OtherComp :type "PrimitiveComponent Object Reference") (NormalImpulse :type "Vector Structure") (Hit :type "HitResult Structure (by ref)"))
  (`KismetSystemLibrary.PrintString` "Hello"))

(fn `UserConstructionScript`)