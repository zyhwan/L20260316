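; Spine trap actor that damages and knocks back the player when its Box component is hit.
; On hit, it casts the other actor to BP_Player, subtracts Damage directly from HP, then launches the character away from the trap with an added upward boost.
; A CanTakeDamage flag and a short Delay act as a cooldown between successive hits.
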(event `self.Box.OnComponentHit`
  (params (HitComponent :type "PrimitiveComponent Object Reference") (OtherActor :type "Actor Object Reference") (OtherComp :type "PrimitiveComponent Object Reference") (NormalImpulse :type "Vector Structure") (Hit :type "HitResult Structure (by ref)"))
  (if (`self.bCanTakeDamage`)
    (bind _asbp_player (cast `/Game/Blueprints/Player/BP_Player` OtherActor))
    (bind _output_get (set `self.BP_Player` _asbp_player))
    (set `/Game/Blueprints/Player/BP_Player.HP` (- (`/Game/Blueprints/Player/BP_Player.HP` _asbp_player) (`self.Damage`)) _output_get)
    (`Character.LaunchCharacter` (`self.BP_Player`) (`KismetMathLibrary.MakeVector` (.x (* (`KismetMathLibrary.Normal` (- (`self.K2_GetActorLocation` (`self.BP_Player`)) (`self.K2_GetActorLocation`))) 1000.0)) (.y (* (`KismetMathLibrary.Normal` (- (`self.K2_GetActorLocation` (`self.BP_Player`)) (`self.K2_GetActorLocation`))) 1000.0)) (+ (.z (* (`KismetMathLibrary.Normal` (- (`self.K2_GetActorLocation` (`self.BP_Player`)) (`self.K2_GetActorLocation`))) 1000.0)) 500.0)) true true)
    (set `self.bCanTakeDamage` false)
    (`KismetSystemLibrary.Delay` 1.0)
    (set `self.bCanTakeDamage` true)))

(fn `UserConstructionScript`)