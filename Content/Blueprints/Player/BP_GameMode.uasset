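; BP_GameMode is a game mode that populates the level with monsters and tracks elapsed game time.
; On BeginPlay it spawns ten BP_Monster actors at random horizontal offsets around the player, starting the music track on each loop pass.
; Tick accumulates game time and prints it against the time limit in Korean debug text.
; Logic to destroy monsters after the limit exists but is disconnected, so it never runs.
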(event `self.ReceiveBeginPlay`
  (bind (_returnvalue_x _returnvalue_y) (`KismetMathLibrary.BreakVector` (`KismetMathLibrary.RandomUnitVector`)))
  (for _ (range 10)
    (`|SpawnActorFromClass` "/Game/Blueprints/Monster/class/BP_Monster.BP_Monster_C" (`KismetMathLibrary.MakeTransform` (+ (* (`KismetMathLibrary.MakeVector` _returnvalue_x _returnvalue_y) 1500.0) (`self.K2_GetActorLocation` (`GameplayStatics.GetPlayerPawn` 0)))) "Undefined" "MultiplyWithRoot" null null)
    (`GameplayStatics.PlaySound2D` "/Game/FreeAtmosGameMusic/wav/Dark_West_3_Canyon_Echoes.Dark_West_3_Canyon_Echoes" 0.05 1.0 0.0 null null)))

(event `self.ReceiveTick`
  (params (DeltaSeconds :type "Float (single-precision)"))
  (bind _output_get (set `self.GameTime` (+ DeltaSeconds (`self.GameTime`))))
  (`KismetSystemLibrary.PrintString` (`KismetTextLibrary.Conv_TextToString` (`|FormatText` "게임 시간 : { 0 } 초 / { 1 } 제한 시간 " (`KismetTextLibrary.Conv_DoubleToText` (/ _output_get 1.0) "HalfToEven") (`self.MaxGameTime`))) true true (struct :`G` 0.66 :`B` 1.0 :`A` 1.0) 0.0))

(fn `UserConstructionScript`)